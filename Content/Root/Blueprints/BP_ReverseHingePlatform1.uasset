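; BP_ReverseHingePlatform1 is a platform that swings on a hinge when gravity swaps.
; SwapGravity drives a FlipFlop that alternately plays and reverses the HINGE timeline, which lerps the whole actor's world rotation from zero to NewRelativeRotation.
; BeginPlay fires the same FlipFlop, so the platform starts by swinging toward the target and the first swap sends it back.
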(event `self.SwapGravity`
  (`/Engine/EditorBlueprintResources/StandardMacros.FlipFlop` :!label _label
    (:`A`
      (bind (_direction _newtrack_0) (`Timeline|HINGE` :!label _label_2)
        (:`Update`
          (`self.K2_SetActorRotation` self (`KismetMathLibrary.RLerp` (struct) (`self.New Relative Rotation`) _newtrack_0) false))))
    (:`B`
      (goto _label_2 :!via `Reverse`))))

(event `self.ReceiveBeginPlay`
  (`parent.ReceiveBeginPlay`)
  (goto _label))

(fn `UserConstructionScript`
  (`parent.UserConstructionScript`))