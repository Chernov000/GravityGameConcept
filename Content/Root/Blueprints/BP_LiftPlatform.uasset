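; BP_LiftPlatform is a platform actor that notifies the player pawn through the BPI_Anchor interface when actors enter or leave its overlap.
; Begin overlap calls Checker and end overlap calls CheckAttraction, both on player pawn 0 without checking which actor overlapped.
; Its Attraction component overlaps, TriggerAnchor and CheckAttraction events are empty, and the graph contains no lift movement.
; Disconnected leftover nodes reference BP_PlatformerChar directly.
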(event `self.ReceiveActorBeginOverlap`
  (params (OtherActor :type "Actor Object Reference"))
  (bind _asbpi_anchor (cast `/Game/Root/Blueprints/BPI_Anchor` (`GameplayStatics.GetPlayerPawn` 0)))
  (`/Game/Root/Blueprints/BPI_Anchor.Checker` _asbpi_anchor))

(event `self.ReceiveActorEndOverlap`
  (params (OtherActor :type "Actor Object Reference"))
  (bind _asbpi_anchor (cast `/Game/Root/Blueprints/BPI_Anchor` (`GameplayStatics.GetPlayerPawn` 0)))
  (`/Game/Root/Blueprints/BPI_Anchor.CheckAttraction` _asbpi_anchor))

(event `self.attraction.OnComponentBeginOverlap`
  (params (OverlappedComponent :type "PrimitiveComponent Object Reference") (OtherActor :type "Actor Object Reference") (OtherComp :type "PrimitiveComponent Object Reference") (OtherBodyIndex :type Integer) (bFromSweep :type Boolean) (SweepResult :type "HitResult Structure (by ref)")))

(event `self.attraction.OnComponentEndOverlap`
  (params (OverlappedComponent :type "PrimitiveComponent Object Reference") (OtherActor :type "Actor Object Reference") (OtherComp :type "PrimitiveComponent Object Reference") (OtherBodyIndex :type Integer)))

(event `/Game/Root/Blueprints/BPI_Anchor.TriggerAnchor`)

(event `/Game/Root/Blueprints/BPI_Anchor.CheckAttraction`)

(fn `UserConstructionScript`
  (`parent.UserConstructionScript`))