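; BP_HingePlatform is a platform actor that toggles between its origin and a closed position each time its SwapGravity event fires.
; A FlipFlop alternately plays and reverses the HINGE timeline, whose track lerps the Platform component's relative location toward CloseddLoc without sweep.
; Despite the hinge name, the live logic only translates the platform; several rotation nodes remain in the graph but are never run.
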(event `self.SwapGravity`
  (`/Engine/EditorBlueprintResources/StandardMacros.FlipFlop`
    (:`A`
      (bind (_direction _newtrack_0) (`Timeline|HINGE` :!label _label)
        (:`Update`
          (`SceneComponent.K2_SetRelativeLocation` (`self.Platform`) (`KismetMathLibrary.VLerp` (0.0 0.0 0.0) (`self.closeddLoc`) _newtrack_0) false false))))
    (:`B`
      (goto _label :!via `Reverse`))))

(fn `UserConstructionScript`
  (`parent.UserConstructionScript`))