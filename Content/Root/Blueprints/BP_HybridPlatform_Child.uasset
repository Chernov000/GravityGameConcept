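; BP_HybridPlatform_Child is a child platform Blueprint that moves its Platform component between its relative origin and EndLoc.
; A Timeline alpha drives the location lerp without sweeping.
; BeginPlay and TriggerAnchor share a FlipFlop, so movement starts at spawn and each anchor trigger alternately stops or resumes it.
; Swap calls Movement, but Movement and SwapGravity have empty bodies here.
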(event `/Game/Root/Blueprints/BPI_GravitySwap.Swap`
  (`self.Movement`))

(event `/Game/Root/Blueprints/BPI_Anchor.TriggerAnchor`
  (`/Engine/EditorBlueprintResources/StandardMacros.FlipFlop` :!label _label
    (:`A`
      (bind (_direction _movementalpha) (`Timeline|Timeline` :!label _label_2)
        (:`Update`
          (`SceneComponent.K2_SetRelativeLocation` (`self.Platform`) (`KismetMathLibrary.VLerp` (0.0 0.0 0.0) (`self.EndLoc`) _movementalpha) false false))))
    (:`B`
      (goto _label_2 :!via `Stop`))))

(event `Movement`)

(event `self.SwapGravity`)

(event `self.ReceiveBeginPlay`
  (`parent.ReceiveBeginPlay`)
  (goto _label))

(fn `UserConstructionScript`
  (`parent.UserConstructionScript`))